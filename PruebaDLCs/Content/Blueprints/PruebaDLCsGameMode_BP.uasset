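; Game mode for what appears to be a DLC test project, applying the player's character and material choices when play begins.
; Sets game-only input, then for each PlayerStart has the Player_BP controller spawn the class from GameInstance_BP at that transform.
; Within the same loop, the game instance's Material index picks gold, basalt or brick for slot 0 of every StaticMeshActor not tagged "Video".
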(event `self.ReceiveBeginPlay`
  (`WidgetBlueprintLibrary.SetInputMode_GameOnly` (`GameplayStatics.GetPlayerController` 0))
  (bind _outactors (`GameplayStatics.GetAllActorsOfClass` "/Script/Engine.PlayerStart"))
  (for _array_element _outactors
    (bind _returnvalue (`self.GetTransform` _array_element))
    (set `self.SpawnTransform` _returnvalue)
    (bind _asgame_instance_bp (cast `/Game/Blueprints/GameInstance_BP` (`GameplayStatics.GetGameInstance`)))
    (bind _output_get (set `self.Game Instance` _asgame_instance_bp))
    (bind _class (`/Game/Blueprints/GameInstance_BP.GetPlayerClass` _output_get))
    (set `self.Model` _class)
    (bind _asplayer_bp (cast `/Game/Blueprints/Player_BP` (`GameplayStatics.GetPlayerController` 0)))
    (`/Game/Blueprints/Player_BP.SpawnCharacter` _asplayer_bp (`self.Model`) _returnvalue)
    (bind _outactors_2 (`GameplayStatics.GetAllActorsOfClass` "/Script/Engine.StaticMeshActor"))
    (switch `int` (`/Game/Blueprints/GameInstance_BP.Material` (`self.Game Instance`))
      (:`0`
        (for _array_element_2 _outactors_2
          (if (not (`self.ActorHasTag` _array_element_2 "Video"))
            (`PrimitiveComponent.SetMaterial` (`StaticMeshActor.StaticMeshComponent` _array_element_2) 0 "/Game/StarterContent/Materials/M_Metal_Gold.M_Metal_Gold"))))
      (:`1`
        (for _array_element_3 _outactors_2
          (if (not (`self.ActorHasTag` _array_element_3 "Video"))
            (`PrimitiveComponent.SetMaterial` (`StaticMeshActor.StaticMeshComponent` _array_element_3) 0 "/Game/StarterContent/Materials/M_Rock_Basalt.M_Rock_Basalt"))))
      (:`2`
        (for _array_element_4 _outactors_2
          (if (not (`self.ActorHasTag` _array_element_4 "Video"))
            (`PrimitiveComponent.SetMaterial` (`StaticMeshActor.StaticMeshComponent` _array_element_4) 0 "/Game/DLCs/EquipoAmarillo/Material/M_Brick_Clay_Old.M_Brick_Clay_Old")))))))

(fn `UserConstructionScript`)