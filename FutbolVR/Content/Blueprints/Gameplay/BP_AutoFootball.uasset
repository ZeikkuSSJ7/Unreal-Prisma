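; BP_AutoFootball is a physics football that kicks itself repeatedly and marks where it hits targets.
; A looping one-second timer calls KickBall, which applies a fixed impulse along world +Y and up.
; When the ball hits an actor tagged "Tageto", it spawns a small BP_Cube at the impact location, zeroes its velocities and returns to the actor location saved at BeginPlay.
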(event `self.ReceiveBeginPlay`
  (set `self.Origin` (`self.K2_GetActorLocation`))
  (`KismetSystemLibrary.K2_SetTimer` null "KickBall" 1.0 true))

(event `self.Football.OnComponentHit`
  (params (HitComponent :type "PrimitiveComponent Object Reference") (OtherActor :type "Actor Object Reference") (OtherComp :type "PrimitiveComponent Object Reference") (NormalImpulse :type "Vector Structure") (Hit :type "HitResult Structure (by ref)"))
  (bind _football (`self.Football`))
  (if (`self.ActorHasTag` OtherActor "Tageto")
    (`|SpawnActorFromClass` "/Game/Blueprints/Gameplay/BP_Cube.BP_Cube_C" (`KismetMathLibrary.MakeTransform` (`.Location` (`GameplayStatics.BreakHitResult` Hit)) (struct) (0.15 0.15 0.15)) "Undefined" "OverrideRootScale" null null)
    (`PrimitiveComponent.SetPhysicsLinearVelocity` _football (0.0 0.0 0.0) false "None")
    (`PrimitiveComponent.SetPhysicsAngularVelocityInDegrees` _football (0.0 0.0 0.0) false "None")
    (`SceneComponent.K2_SetWorldLocation` _football (`self.Origin`) false false)))

(fn `KickBall`
  (`PrimitiveComponent.AddImpulse` (`self.Football`) (* (`KismetMathLibrary.MakeVector` 0.0 1.0 1.0) 10000.0) "None" false))

(fn `UserConstructionScript`)