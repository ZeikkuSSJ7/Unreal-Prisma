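; BP_OculusHand is an Oculus hand-tracking component that detects grab gestures and fires OnGrab and OnRelease events when the state changes.
; After a short delay it waits for high tracking confidence, polling by timer if needed, then caches fingertip bone names and enables tick.
; Each tick maps average fingertip-to-wrist distance to an inverted, clamped grab axis, so curled fingers exceeding the threshold count as grabbing.
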(event `self.ReceiveBeginPlay`
  (`KismetSystemLibrary.Delay` 1.0)
  (if (`|EnumEquality` (`OculusInputFunctionLibrary.GetTrackingConfidence` (`self.MeshType`)) "High")
    (for _index (range (`self.GetNumBones`)) :!label _label
      (bind _returnvalue (`self.GetBoneName` _index))
      (if (`KismetStringLibrary.Contains` (`KismetStringLibrary.ToLower` (`KismetStringLibrary.Conv_NameToString` _returnvalue)) "tip")
        (`KismetArrayLibrary.Array_Add` (`self.FingerTips`) _returnvalue)
        (`KismetSystemLibrary.PrintString` (`KismetStringLibrary.Conv_NameToString` _returnvalue))))
    (`self.SetComponentTickEnabled` true)
    (else
      (bind _returnvalue_2 (`KismetSystemLibrary.K2_SetTimerDelegate` (delegate `CustomEvent_0`) 0.1 true)))))

(event `CustomEvent_0`
  (if (`|EnumEquality` (`OculusInputFunctionLibrary.GetTrackingConfidence` (`self.MeshType`)) "High")
    (`KismetSystemLibrary.K2_ClearAndInvalidateTimerHandle` (stale `self.ReceiveBeginPlay` _returnvalue_2))
    (goto _label)))

(event `self.ReceiveTick`
  (params (DeltaSeconds :type "Float (single-precision)"))
  (if (`self.DetectGrabbing`)
    (if (not (`self.bGrabbed`))
      (`self.OnGrab`)
      (set `self.bGrabbed` true))
    (elif (`self.bGrabbed`)
      (`self.OnRelease`)
      (set `self.bGrabbed` false))))

(fn `DetectGrabbing`
  (returns (Grabbed :type Boolean))
  (locals (Distances :type "Array of Float (double-precision)") (DistanceTotal :type "Float (double-precision)") (DistanceAverage :type "Float (double-precision)"))
  (for _array_element (`self.FingerTips`)
    (bind _returnvalue (`self.GetBoneLocationByName` _array_element "WorldSpace"))
    (bind _returnvalue_2 (`self.GetBoneLocationByName` (`self.WristBone`) "WorldSpace"))
    (`KismetArrayLibrary.Array_Add` (`local.Distances`) (`KismetMathLibrary.Abs` (`KismetMathLibrary.VSize` (- _returnvalue_2 _returnvalue)))))
  (for _array_element_2 (`local.Distances`)
    (set `local.DistanceTotal` (+ _array_element_2 (`local.DistanceTotal`))))
  (if (== (`local.DistanceTotal`) 0.0)
    (return false)
    (else
      (bind _output_get (set `local.DistanceAverage` (/ (`local.DistanceTotal`) (`KismetMathLibrary.Conv_IntToDouble` (`KismetArrayLibrary.Array_Length` (`local.Distances`))))))
      (bind _output_get_2 (set `self.GrabAxis` (`KismetMathLibrary.MapRangeClamped` _output_get 7.8 16.9 1.0)))
      (if (> _output_get_2 (`self.GradThreshold`))
        (return true)
        (else
          (return false))))))