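; Oculus hand-tracking actor for one hand that points at and clicks UI widgets with a visible laser.
; The Hand setting picks the motion source, hand mesh and skeleton, and gives each hand its own virtual user index.
; Each tick, a high-confidence valid pointer pose moves the WidgetInteraction and spline, stretching the spline mesh to any blocking hit and otherwise collapsing it.
; Press and Released events send left-mouse pointer key input.
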(event `self.ReceiveBeginPlay`
  (bind _widgetinteraction (`self.WidgetInteraction`))
  (switch `EControllerHand` (`self.Hand`)
    (:`Left`
      (set `WidgetInteractionComponent.VirtualUserIndex` 0 _widgetinteraction))
    (:`Right`
      (set `WidgetInteractionComponent.VirtualUserIndex` 1 _widgetinteraction))))

(event `self.ReceiveTick`
  (params (DeltaSeconds :type "Float (single-precision)"))
  (bind _returnvalue (`self.GetTransform`))
  (bind (_returnvalue_location _returnvalue_rotation) (`KismetMathLibrary.BreakTransform` (`OculusInputFunctionLibrary.GetPointerPose` (`self.GetOculusHand`))))
  (bind (_bblockinghit _binitialoverlap _time _distance _location) (`GameplayStatics.BreakHitResult` (`WidgetInteractionComponent.GetLastHitResult` (`self.WidgetInteraction`))))
  (switch `ETrackingConfidence` (`OculusInputFunctionLibrary.GetTrackingConfidence` (`self.GetOculusHand`))
    (:`Low`
      (`self.CollapseSpline`))
    (:`High`
      (if (`OculusInputFunctionLibrary.IsPointerPoseValid` (`self.GetOculusHand`))
        (`SceneComponent.K2_SetWorldLocationAndRotation` (`self.Spline`) (`KismetMathLibrary.TransformLocation` _returnvalue _returnvalue_location) (`KismetMathLibrary.TransformRotation` _returnvalue _returnvalue_rotation) false false)
        (`SceneComponent.K2_SetWorldLocationAndRotation` (`self.WidgetInteraction`) (`KismetMathLibrary.TransformLocation` _returnvalue _returnvalue_location) (`KismetMathLibrary.TransformRotation` _returnvalue _returnvalue_rotation) false false)
        (if _bblockinghit
          (`SplineComponent.SetLocationAtSplinePoint` (`self.Spline`) 1 _location "World" true)
          (`self.UpdateSplineMesh`)
          (else
            (`self.CollapseSpline`)))
        (else
          (`self.CollapseSpline`))))))

(event `Press`
  (`WidgetInteractionComponent.PressPointerKey` (`self.WidgetInteraction`) "LeftMouseButton"))

(event `Released`
  (`WidgetInteractionComponent.ReleasePointerKey` (`self.WidgetInteraction`) "LeftMouseButton"))

(fn `CollapseSpline`
  (`SplineComponent.SetLocationAtSplinePoint` (`self.Spline`) 1 (`SplineComponent.GetLocationAtSplinePoint` (`self.Spline`) 0 "World") "World" true)
  (`self.UpdateSplineMesh`))

(fn `GetOculusHand`
  (returns (ReturnValue :type "EOculusHandType Enum"))
  (return (select `EControllerHand` (`self.Hand`) :`Left` "HandLeft" :`Right` "HandRight" :!type "EOculusHandType Enum")))

(fn `UpdateSplineMesh`
  (bind _spline (`self.Spline`))
  (bind (_location _tangent) (`SplineComponent.GetLocationAndTangentAtSplinePoint` _spline 0 "Local"))
  (bind (_location_2 _tangent_2) (`SplineComponent.GetLocationAndTangentAtSplinePoint` _spline 1 "Local"))
  (`SplineMeshComponent.SetStartAndEnd` (`self.SplineMesh`) _location _tangent _location_2 _tangent_2 true))

(fn `UserConstructionScript`
  (bind _returnvalue (`self.GetOculusHand`))
  (bind _oculushand (`self.OculusHand`))
  (set `MotionControllerComponent.MotionSource` (`|GetEnumeratorName` (`self.Hand`)) (`self.MotionController`))
  (set `OculusHandComponent.MeshType` _returnvalue _oculushand)
  (set `OculusHandComponent.SkeletonType` _returnvalue _oculushand))