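; VR pawn that sets floor-level tracking and spawns attached left and right Hand_BP actors on BeginPlay.
; Left and right index pinch inputs forward press and release to the matching hand.
; The Menu input prints GetMenuTransform, spawns a Projectile actor there and stores it as Menu.
; GetMenuTransform holds only an unconnected transform calculation based on the right controller's flattened forward vector.
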(event `self.ReceiveBeginPlay`
  (bind _returnvalue (`KismetMathLibrary.MakeTransform` (0.0 0.0 0.0)))
  (`|ExecutionSequence`
    (:`then_0`
      (`HeadMountedDisplayFunctionLibrary.SetTrackingOrigin` "Floor"))
    (:`then_1`
      (`|ExecutionSequence`
        (:`then_0`
          (bind _returnvalue_2 (`|SpawnActorFromClass` "/Game/Blueprints/Hand_BP.Hand_BP_C" _returnvalue "AlwaysSpawn" "OverrideRootScale" self "Left" null))
          (bind _output_get (set `self.Left` _returnvalue_2))
          (`self.K2_AttachToActor` _output_get self "None" "SnapToTarget" "SnapToTarget" "KeepWorld" false))
        (:`then_1`
          (bind _returnvalue_3 (`|SpawnActorFromClass` "/Game/Blueprints/Hand_BP.Hand_BP_C" _returnvalue "AlwaysSpawn" "OverrideRootScale" self "Right" null))
          (bind _output_get_2 (set `self.Right` _returnvalue_3))
          (`self.K2_AttachToActor` _output_get_2 self "None" "SnapToTarget" "SnapToTarget" "KeepWorld" false))))))

(event `InputAction|LeftIndexPinch`
  (params (Key :type "Key Structure"))
  (bind _left (`self.Left`))
  (:`Pressed`
    (`/Game/Blueprints/Hand_BP.Press` _left))
  (:`Released`
    (`/Game/Blueprints/Hand_BP.Released` _left)))

(event `InputAction|Menu`
  (params (Key :type "Key Structure"))
  (bind _motioncontroller (`/Game/Blueprints/Hand_BP.MotionController` (`self.Right`)))
  (bind _returnvalue (`SceneComponent.K2_GetComponentLocation` _motioncontroller))
  (bind _returnvalue_2 (+ _returnvalue (* (`KismetMathLibrary.MakeVector` (.x (`SceneComponent.GetForwardVector` _motioncontroller)) (.y (`SceneComponent.GetForwardVector` _motioncontroller))) 100.0)))
  (bind _returnvalue_3 (`KismetMathLibrary.MakeTransform` _returnvalue_2 (`KismetMathLibrary.FindLookAtRotation` _returnvalue _returnvalue_2)))
  (:`Pressed`
    (`KismetSystemLibrary.PrintString` (`KismetStringLibrary.Conv_TransformToString` _returnvalue_3))
    (bind _returnvalue_4 (`|SpawnActorFromClass` "/Game/VRTemplate/Blueprints/Projectile.Projectile_C" _returnvalue_3 "AlwaysSpawn" "OverrideRootScale" null null))
    (set `self.Menu` _returnvalue_4)))

(event `InputAction|RightIndexPinch`
  (params (Key :type "Key Structure"))
  (bind _right (`self.Right`))
  (:`Pressed`
    (`/Game/Blueprints/Hand_BP.Press` _right))
  (:`Released`
    (`/Game/Blueprints/Hand_BP.Released` _right)))

(fn `UserConstructionScript`)