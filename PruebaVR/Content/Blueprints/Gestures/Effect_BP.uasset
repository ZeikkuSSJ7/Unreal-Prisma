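; Effect_BP is an actor in the Gestures folder that plays fire, water or magic particle effects at its own location and rotation.
; Three custom events, SpawnFire, SpawnWater and SpawnMagic, each spawn their own storm or magic-circle emitter.
; Each event destroys its emitter after a short delay, with a DoOnce gate that blocks retriggering until that cleanup resets it.
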(event `SpawnFire`
  (`/Engine/EditorBlueprintResources/StandardMacros.DoOnce` false :!label _label
    (:`Completed`
      (bind _returnvalue (`GameplayStatics.SpawnEmitterAtLocation` "/Game/FXVarietyPack/Particles/P_ky_fireStorm.P_ky_fireStorm" (`self.K2_GetActorLocation`) (`self.K2_GetActorRotation`)))
      (`KismetSystemLibrary.Delay` 2.0)
      (`ActorComponent.K2_DestroyComponent` _returnvalue)
      (goto _label :!via `Reset`))))

(event `SpawnWater`
  (`/Engine/EditorBlueprintResources/StandardMacros.DoOnce` false :!label _label_2
    (:`Completed`
      (bind _returnvalue (`GameplayStatics.SpawnEmitterAtLocation` "/Game/FXVarietyPack/Particles/P_ky_aquaStorm.P_ky_aquaStorm" (`self.K2_GetActorLocation`) (`self.K2_GetActorRotation`)))
      (`KismetSystemLibrary.Delay` 2.0)
      (`ActorComponent.K2_DestroyComponent` _returnvalue)
      (goto _label_2 :!via `Reset`))))

(event `SpawnMagic`
  (`/Engine/EditorBlueprintResources/StandardMacros.DoOnce` false :!label _label_3
    (:`Completed`
      (bind _returnvalue (`GameplayStatics.SpawnEmitterAtLocation` "/Game/FXVarietyPack/Particles/P_ky_magicCircle1.P_ky_magicCircle1" (`self.K2_GetActorLocation`) (`self.K2_GetActorRotation`)))
      (`KismetSystemLibrary.Delay` 2.0)
      (`ActorComponent.K2_DestroyComponent` _returnvalue)
      (goto _label_3 :!via `Reset`))))

(fn `UserConstructionScript`)