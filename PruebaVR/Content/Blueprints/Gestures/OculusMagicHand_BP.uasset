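; Oculus hand Blueprint that records static hand poses as named gestures and recognises them at runtime.
; RecordGesture saves component-space bone locations under unique names in a SaveGame slot, loaded at BeginPlay.
; A looping timer finds the first saved gesture with every bone within Threshold distance and fires OnGestureRecognised when it changes.
; DeleteGesture finds the matching index, but its removal and save nodes are never executed.
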(event `self.ReceiveBeginPlay`
  (set `self.Gesture` (`/Game/Blueprints/Gestures/SaveGameGesture_BP.Gesture` (`self.LoadGestures`)))
  (`KismetSystemLibrary.K2_SetTimerDelegate` (delegate `DetectGestures`) (`self.RefreshRate`) true))

(event `DetectGestures`
  (bind (_result _gesture) (`self.GetCurrentGesture`))
  (if _result
    (if (not (`self.EqualGesture` _gesture (`self.CurrentGesture`)))
      (bind _output_get (set `self.CurrentGesture` _gesture))
      (`self.OnGestureRecognised` (`.GestureName_2_7A52E7F4432BAC0F44C9F3AA012D1BDB` (break `/Game/Blueprints/Gestures/SGesture` _output_get))))))

(fn `Delete Gesture`
  (params (`Gesture Name` :type String))
  (locals (GestureSaveGame :type "/Game/Blueprints/Gestures/SaveGameGesture_BP Object Reference"))
  (bind _output_get (set `local.GestureSaveGame` (`self.LoadGestures`)))
  (for (_array_element _array_index) (`/Game/Blueprints/Gestures/SaveGameGesture_BP.Gesture` _output_get)
    (if (`KismetStringLibrary.EqualEqual_StrStr` (`.GestureName_2_7A52E7F4432BAC0F44C9F3AA012D1BDB` (break `/Game/Blueprints/Gestures/SGesture` _array_element)) `Gesture Name`)
      (set `self.Index` _array_index))))

(fn `DoesGestureExist`
  (params (SaveGameGesture :type "/Game/Blueprints/Gestures/SaveGameGesture_BP Object Reference") (GestureName :type String))
  (returns (Result :type Boolean))
  (for _array_element (`/Game/Blueprints/Gestures/SaveGameGesture_BP.Gesture` SaveGameGesture)
    (if (`KismetStringLibrary.EqualEqual_StrStr` (`.GestureName_2_7A52E7F4432BAC0F44C9F3AA012D1BDB` (break `/Game/Blueprints/Gestures/SGesture` _array_element)) GestureName)
      (return true)))
  (return false))

(fn `EqualGesture`
  (params (A :type "/Game/Blueprints/Gestures/SGesture Structure") (B :type "/Game/Blueprints/Gestures/SGesture Structure"))
  (returns (Result :type Boolean))
  (bind (_gesturename _bonelocations) (break `/Game/Blueprints/Gestures/SGesture` B))
  (bind (_gesturename_2 _bonelocations_2) (break `/Game/Blueprints/Gestures/SGesture` A))
  (return (and (`KismetStringLibrary.EqualEqual_StrStr` _gesturename_2 _gesturename) (`KismetArrayLibrary.Array_Identical` _bonelocations_2 _bonelocations))))

(fn `GetCurrentGesture`
  (returns (Result :type Boolean) (Gesture :type "/Game/Blueprints/Gestures/SGesture Structure"))
  (bind _bvalidgesture (`self.bValidGesture`))
  (for _array_element (`self.Gesture`)
    (for (_array_element_2 _array_index) (`.BoneLocations_6_6E5DE7494A0C56BD22D30F834EC4DBF4` (break `/Game/Blueprints/Gestures/SGesture` _array_element))
      (bind _returnvalue (`self.GetBoneLocationByName` (`self.GetBoneName` _array_index) "ComponentSpace"))
      (if (> (`KismetMathLibrary.Abs` (`KismetMathLibrary.VSize` (- _returnvalue _array_element_2))) (`self.Threshold`))
        (set `self.bValidGesture` false)))
    (if _bvalidgesture
      (return _bvalidgesture _array_element)
      (else
        (set `self.bValidGesture` true)))))

(fn `LoadGestures`
  (returns (Output :type "/Game/Blueprints/Gestures/SaveGameGesture_BP Object Reference"))
  (bind _returnvalue (`GameplayStatics.DoesSaveGameExist` (`self.GestureGameSlot`)))
  (if _returnvalue
    (bind _returnvalue_2 (`GameplayStatics.LoadGameFromSlot` (`self.GestureGameSlot`)))
    (bind _assave_game_gesture_bp (cast `/Game/Blueprints/Gestures/SaveGameGesture_BP` _returnvalue_2))
    (return _assave_game_gesture_bp)
    (else
      (bind _returnvalue_3 (`GameplayStatics.CreateSaveGameObject` "/Game/Blueprints/Gestures/SaveGameGesture_BP.SaveGameGesture_BP_C"))
      (return _returnvalue_3))))

(fn `RecordGesture`
  (params (GestureName :type String))
  (locals (BoneLocations :type "Array of Vector Structure") (GestureSaveGame :type "/Game/Blueprints/Gestures/SaveGameGesture_BP Object Reference"))
  (bind _output_get (set `local.GestureSaveGame` (`self.LoadGestures`)))
  (if (not (`self.DoesGestureExist` _output_get GestureName))
    (for _index (range (`self.GetNumBones`))
      (bind _returnvalue (`self.GetBoneLocationByName` (`self.GetBoneName` _index) "ComponentSpace"))
      (`KismetArrayLibrary.Array_Add` (`local.BoneLocations`) _returnvalue))
    (`KismetArrayLibrary.Array_Add` (`/Game/Blueprints/Gestures/SaveGameGesture_BP.Gesture` (`local.GestureSaveGame`)) (make `/Game/Blueprints/Gestures/SGesture` (`local.GestureName`) (`local.BoneLocations`)))
    (`GameplayStatics.SaveGameToSlot` (`local.GestureSaveGame`) (`self.GestureGameSlot`))))