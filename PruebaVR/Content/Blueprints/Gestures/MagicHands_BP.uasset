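; MagicHands_BP is a VR hand-gesture spellcasting Blueprint that spawns elemental effects from recognised hand poses.
; On BeginPlay it sets floor-level tracking and binds both hand components' gesture-recognised events to one handler.
; That handler maps Rock, Point and Ok gestures to fire, magic and water spawns on the Effect object.
; Debug keys record a gesture per hand or delete it from both, printing Spanish confirmations.
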(event `self.ReceiveBeginPlay`
  (`HeadMountedDisplayFunctionLibrary.SetTrackingOrigin` "Floor")
  (add `/Game/Blueprints/Gestures/OculusMagicHand_BP.OnGestureRecognised` (`self.Left`) (`|CreateDelegate` :!event `GestureRecognised`))
  (add `/Game/Blueprints/Gestures/OculusMagicHand_BP.OnGestureRecognised` (`self.Right`) (`|CreateDelegate` :!event `GestureRecognised`)))

(event `GestureRecognised`
  (params (GestureName :type String))
  (bind _effect (`self.Effect`))
  (switch `string` GestureName
    (:`Rock`
      (`/Game/Blueprints/Gestures/Effect_BP.SpawnFire` _effect))
    (:`Point`
      (`/Game/Blueprints/Gestures/Effect_BP.SpawnMagic` _effect))
    (:`Ok`
      (`/Game/Blueprints/Gestures/Effect_BP.SpawnWater` _effect))))

(event `Key|R`
  (params (Key :type "Key Structure"))
  (:`Pressed`
    (`/Game/Blueprints/Gestures/OculusMagicHand_BP.RecordGesture` (`self.Right`) (`self.GestureName`))
    (`KismetSystemLibrary.PrintString` "He recordado la derecha")))

(event `Key|L`
  (params (Key :type "Key Structure"))
  (:`Pressed`
    (`/Game/Blueprints/Gestures/OculusMagicHand_BP.RecordGesture` (`self.Left`) (`self.GestureName`))
    (`KismetSystemLibrary.PrintString` "He recordado la izquierda")))

(event `Key|D`
  (params (Key :type "Key Structure"))
  (:`Pressed`
    (`/Game/Blueprints/Gestures/OculusMagicHand_BP.Delete Gesture` (`self.Left`) (`self.GestureName`))
    (`/Game/Blueprints/Gestures/OculusMagicHand_BP.Delete Gesture` (`self.Right`) (`self.GestureName`))
    (`KismetSystemLibrary.PrintString` "He borrado")))

(fn `MagicHands_BP_AutoGenFunc`
  (params (GestureName :type String)))

(fn `UserConstructionScript`)