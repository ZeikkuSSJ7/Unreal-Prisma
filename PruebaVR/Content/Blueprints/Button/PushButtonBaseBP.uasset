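; Base Blueprint for a physical push button, pressed by an overlapping fingertip component, that plays sounds and notifies listed actors on press.
; The construction script derives travel markers and the trigger box from the mesh bounds.
; Tick projects fingertip depth onto the button axis to slide the mesh, interpolating back when untouched.
; Separate press and release thresholds plus a delayed DoOnce reset prevent retriggers, and Tick switches off after idle.
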(event OnComponentBeginOverlap(Box)
  (params (OverlappedComponent :type Primitive%20Component%20Object%20Reference) (OtherActor :type Actor%20Object%20Reference) (OtherComp :type Primitive%20Component%20Object%20Reference) (OtherBodyIndex :type Integer) (bFromSweep :type Boolean) (SweepResult :type Hit%20Result%20Structure%20%28by%20ref%29))
  ;[1 1 1] Overlaps with pointing fingertip
  (Variables|Default|SetFingerTip OtherComp)
  (Actor|Tick|SetActorTickEnabled true)
  (CallFunction|ForceTick))

(event OnComponentEndOverlap(Box)
  (params (OverlappedComponent :type Primitive%20Component%20Object%20Reference) (OtherActor :type Actor%20Object%20Reference) (OtherComp :type Primitive%20Component%20Object%20Reference) (OtherBodyIndex :type Integer))
  ;[1 1 1] Overlaps with pointing fingertip
  (if (== OtherComp (Variables|Default|GetFingerTip))
    (CallFunction|ForceTick)
    (Variables|Default|SetFingerTip 0)
    (Utilities|FlowControl|RetriggerableDelay 3.0)
    (Utilities|IsValid (Variables|Default|GetFingerTip)
      (:Is%20Not%20Valid
        (Actor|Tick|SetActorTickEnabled false)))))

(event Custom|Force%20Tick
  ;[1 1 1] Tick
  (Variables|Default|SetCurrentPushedAmount (CallFunction|GetPushedAmount))
  (|UpdateButtonLocation)
  (if (|({26BD75D0-4264-6CD8-9CC2-40B0526D647B}<=0.900000))
    (if (Variables|Default|GetButtonIsDown)
      (CallFunction|ButtonReleased))
    (elif (not (|({26BD75D0-4264-6CD8-9CC2-40B0526D647B}<0.999999)))
      (Utilities|FlowControl|DoOnce false
        (:Completed
          (CallFunction|ButtonPressed))))))

(event Custom|ButtonReleased
  ;[1 1 1] On button press/release logic
  (Variables|Default|SetButtonIsDown false)
  (Audio|PlaySoundatLocation (Variables|Default|GetPressOutSound) (Transformation|GetWorldLocation) "0, 0, 0" 1.0 1.0 0.0 0 0 0)
  (Utilities|FlowControl|Delay 0.2)
  (CallFunction|ResetButton))

(event Custom|ButtonPressed
  ;[1 1 1] On button press/release logic
  (if (not (Variables|Default|GetButtonIsDown))
    (Variables|Default|SetButtonIsDown true)
    (Audio|PlaySoundatLocation (Variables|Default|GetPressInSound) (Transformation|GetWorldLocation) "0, 0, 0" 1.0 1.0 0.0 0 0 0)
    (Default|CallOnButtonPress)
    (for _array_element (Variables|Default|GetActorsToActionOnPress)
      (Class|IsButtonableInterface|ButtonAction(Message) _array_element (Variables|Default|GetActionName)))))

(event Custom|ResetButton
  ;[1 1 1] Tick
  (Utilities|FlowControl|DoOnce false) ; enters at Reset
)

(event EventTick
  (params (DeltaSeconds :type Float%20%28single-precision%29))
  ;[1 1 1] Tick
  (Variables|Default|SetCurrentPushedAmount (CallFunction|GetPushedAmount))
  (|UpdateButtonLocation)
  (if (|({26BD75D0-4264-6CD8-9CC2-40B0526D647B}<=0.900000))
    (if (Variables|Default|GetButtonIsDown)
      (CallFunction|ButtonReleased))
    (elif (not (|({26BD75D0-4264-6CD8-9CC2-40B0526D647B}<0.999999)))
      (Utilities|FlowControl|DoOnce false
        (:Completed
          (CallFunction|ButtonPressed))))))

(event EventBeginPlay
  (bind _attachto (Variables|Default|GetAttachTo))
  ;[1 1 1] If there is an attatch point than attatch to that point
  (Utilities|IsValid _attachto
    (:Is%20Valid
      (Transformation|AttachComponentToComponent (Variables|Default|GetDefaultSceneRoot) _attachto "None" "SnapToTarget" "SnapToTarget" "SnapToTarget" true))))

(fn ConstructionScript
  (bind _buttonmesh (Variables|Default|GetButtonMesh))
  (bind _returnvalue (StaticMesh|GetBounds _buttonmesh))
  (LocalVariables|SetExtentZ (.z (.boxextent (StaticMesh|GetBounds (Variables|Default|GetButtonMesh)))))
  (Components|StaticMesh|SetStaticMesh (Variables|Default|GetMesh) (Variables|Default|GetButtonMesh))
  (Transformation|SetRelativeLocation (Variables|Default|GetPushTo) (Math|Vector|MakeVector 0.0 0.0 (|PushToZ (LocalVariables|GetExtentZ))) false false)
  (Transformation|SetRelativeLocation (Variables|Default|GetPushFrom) (Math|Vector|MakeVector 0.0 0.0 (|PushFromZ (LocalVariables|GetExtentZ))) false false)
  (Transformation|SetRelativeLocation (Variables|Default|GetBox) (Math|Vector|MakeVector 0.0 0.0 (.z (Variables|/Script/Engine.SceneComponent|GetRelativeLocation (Variables|Default|GetPushFrom)))) false false)
  (Components|Box|SetBoxExtent (Variables|Default|GetBox) (Math|Vector|MakeVector (.x (.boxextent _returnvalue)) (.y (.boxextent _returnvalue)) (|BoxExtentZ)) false))

(fn GetPushedAmount
  (Utilities|IsValid (Variables|Default|GetFingerTip)
    (:Is%20Valid
      (return (Math|Float|MapRangeClamped (Math|Vector|DotProduct (- (Transformation|GetWorldLocation (Variables|Default|GetFingerTip)) (Transformation|GetWorldLocation (Variables|Default|GetPushFrom))) (* (Math|Vector|GetUpVector (Variables|Default|GetMesh)) -1.0)) 0.0 (Math|Vector|Distance(Vector) (Transformation|GetWorldLocation (Variables|Default|GetPushTo)) (Transformation|GetWorldLocation (Variables|Default|GetPushFrom))) 0.0 1.0)))
    (:Is%20Not%20Valid
      (return (Math|Interpolation|FInterpTo (Variables|Default|GetCurrentPushedAmount) 0.0 (Utilities|Time|GetWorldDeltaSeconds) (Variables|Default|GetRetractRate))))))