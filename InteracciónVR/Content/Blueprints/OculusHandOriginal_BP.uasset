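; Oculus hand Blueprint that detects finger gestures and calls OnTeleport when a pointing pose closes directly into a fist.
; Each tick, IsFingerDown compares index, middle, ring and pinky tip bones against per-finger sockets using a distance threshold to update down flags.
; Those flags track pointing (only index raised), and any pose other than pointing clears that state.
; IsFingerDown always draws debug points, including at the sockets.
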(event `self.ReceiveTick`
  (params (DeltaSeconds :type "Float (single-precision)"))
  (`|ExecutionSequence`
    (:`then_0`
      (bind _returnvalue (`self.IsFingerDown` (`self.IndexTipBone`) (`self.IndexFingerSocket`)))
      (if _returnvalue
        (if (not (`self.bIndexDown`))
          (set `self.bIndexDown` (not (`self.bIndexDown`)) :!label _label))
        (elif (`self.bIndexDown`)
          (goto _label))))
    (:`then_1`
      (bind _returnvalue_2 (`self.IsFingerDown` (`self.MiddleTipBone`) (`self.MiddleFingerSocket`)))
      (if _returnvalue_2
        (if (not (`self.bMiddleDown`))
          (set `self.bMiddleDown` (not (`self.bMiddleDown`)) :!label _label_2))
        (elif (`self.bMiddleDown`)
          (goto _label_2))))
    (:`then_2`
      (bind _returnvalue_3 (`self.IsFingerDown` (`self.RingTipBone`) (`self.RingFingerSocket`)))
      (if _returnvalue_3
        (if (not (`self.bRingDown`))
          (set `self.bRingDown` (not (`self.bRingDown`)) :!label _label_3))
        (elif (`self.bRingDown`)
          (goto _label_3))))
    (:`then_3`
      (bind _returnvalue_4 (`self.IsFingerDown` (`self.PinkyTipBone`) (`self.PinkyFingerSocket`)))
      (if _returnvalue_4
        (if (not (`self.bPinkyDown`))
          (set `self.bPinkyDown` (not (`self.bPinkyDown`)) :!label _label_4))
        (elif (`self.bPinkyDown`)
          (goto _label_4))))
    (:`then_4`
      (if (and (not (`self.bIndexDown`)) (`self.bMiddleDown`) (`self.bRingDown`) (`self.bPinkyDown`))
        (if (not (`self.bWasPointing`))
          (set `self.bWasPointing` true))
        (elif (and (`self.bIndexDown`) (`self.bMiddleDown`) (`self.bRingDown`) (`self.bPinkyDown`))
          (if (`self.bWasPointing`)
            (`self.OnTeleport`))
          (set `self.bWasPointing` false)
          (else
            (set `self.bWasPointing` false)))))))

(fn `IsFingerDown`
  (params (BoneName :type Name) (SocketName :type Name))
  (returns (ReturnValue :type Boolean))
  (bind _returnvalue (`self.GetSocketLocation` SocketName))
  (bind _returnvalue_2 (`self.GetBoneLocationByName` BoneName "WorldSpace"))
  (if true
    (`KismetSystemLibrary.DrawDebugPoint` (0.0 0.0 0.0) 20.0 (struct :`R` 1.0 :`A` 1.0) 0.1)
    (`KismetSystemLibrary.DrawDebugPoint` _returnvalue 20.0 (struct :`G` 1.0 :`B` 0.02342 :`A` 1.0) 0.1))
  (return (< (`KismetMathLibrary.Abs` (`KismetMathLibrary.VSize` (- _returnvalue_2 _returnvalue))) (`self.Threshold`))))