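; Effect_BP is an effect spawner actor in the Gestures folder, with separate events for fire, water, magic and lightning particle effects.
; Each event spawns its emitter 300 units along world X from the actor, using the actor's rotation, and stores it in a shared Particles variable.
; Each DoOnce resets right after spawning, so repeated calls are not blocked.
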(event `SpawnFire`
  (`/Engine/EditorBlueprintResources/StandardMacros.DoOnce` false :!label _label
    (:`Completed`
      (bind _returnvalue (`GameplayStatics.SpawnEmitterAtLocation` "/Game/FXVarietyPack/Particles/P_ky_fireStorm.P_ky_fireStorm" (+ (`self.K2_GetActorLocation`) (300.0 0.0 0.0)) (`self.K2_GetActorRotation`)))
      (set `self.Particles` _returnvalue)
      (goto _label :!via `Reset`))))

(event `SpawnWater`
  (`/Engine/EditorBlueprintResources/StandardMacros.DoOnce` false :!label _label_2
    (:`Completed`
      (bind _returnvalue (`GameplayStatics.SpawnEmitterAtLocation` "/Game/FXVarietyPack/Particles/P_ky_aquaStorm.P_ky_aquaStorm" (+ (`self.K2_GetActorLocation`) (300.0 0.0 0.0)) (`self.K2_GetActorRotation`)))
      (set `self.Particles` _returnvalue)
      (goto _label_2 :!via `Reset`))))

(event `SpawnMagic`
  (`/Engine/EditorBlueprintResources/StandardMacros.DoOnce` false :!label _label_3
    (:`Completed`
      (bind _returnvalue (`GameplayStatics.SpawnEmitterAtLocation` "/Game/FXVarietyPack/Particles/P_ky_magicCircle1.P_ky_magicCircle1" (+ (`self.K2_GetActorLocation`) (300.0 0.0 0.0)) (`self.K2_GetActorRotation`)))
      (set `self.Particles` _returnvalue)
      (goto _label_3 :!via `Reset`))))

(event `SpawnLight`
  (`/Engine/EditorBlueprintResources/StandardMacros.DoOnce` false :!label _label_4
    (:`Completed`
      (bind _returnvalue (`GameplayStatics.SpawnEmitterAtLocation` "/Game/FXVarietyPack/Particles/P_ky_lightning1.P_ky_lightning1" (+ (`self.K2_GetActorLocation`) (300.0 0.0 0.0)) (`self.K2_GetActorRotation`)))
      (set `self.Particles` _returnvalue)
      (goto _label_4 :!via `Reset`))))

(fn `UserConstructionScript`)